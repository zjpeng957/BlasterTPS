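; Floating damage number actor in the ability system's cue assets, showing a damage value through a widget component.
; On BeginPlay it casts the component's widget to WBP_DamageText, writes DamageValue into its text and plays the pop animation.
; It also prints the value as debug output, then destroys itself after a short delay.
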(event EventBeginPlay
  (bind _damagevalue (Variables|Default|GetDamageValue))
  (bind _returnvalue (Utilities|Text|ToText(Float) _damagevalue "HalfToEven"))
  (bind _aswbp_damage_text (Utilities|Casting|CastToWBP_DamageText (UserInterface|GetUserWidgetObject (Variables|Default|GetWidget))))
  (Development|PrintText _returnvalue)
  (Rendering|Components|TextRender|SetText (Variables|/Game/BluePrints/HUD/WBP_DamageText.WBP_DamageText_C|GetDamageText _aswbp_damage_text) _returnvalue)
  (UserInterface|Animation|PlayAnimation _aswbp_damage_text (Variables|/Game/BluePrints/HUD/WBP_DamageText.WBP_DamageText_C|GetAnimPop _aswbp_damage_text) 0.0 1 "Forward" 1.0 false)
  (Utilities|FlowControl|RetriggerableDelay 1.0)
  (Actor|DestroyActor))

(fn ConstructionScript)